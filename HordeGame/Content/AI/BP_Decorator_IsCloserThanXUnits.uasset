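; Behavior tree decorator that passes when the controlled pawn is within a set distance of a target actor.
; The target is read from a configurable blackboard key, and the straight-line distance between the two actor locations is compared to MaxDistance, inclusive.
; The check fails when the blackboard actor is invalid.
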(fn PerformConditionCheckAI
  (params (OwnerController :type AI%20Controller%20Object%20Reference) (ControlledPawn :type Pawn%20Object%20Reference))
  (bind _blackboard_key (Variables|Default|GetBlackboard%20Key))
  (bind _returnvalue (AI|BehaviorTree|GetBlackboardValueasActor _blackboard_key))
  (Utilities|IsValid _returnvalue
    (:Is%20Valid
      (return (<= (Math|Vector|VectorLength (- (Transformation|GetActorLocation ControlledPawn) (Transformation|GetActorLocation _returnvalue))) (Variables|Default|GetMaxDistance))))
    (:Is%20Not%20Valid
      (return false))))