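; Behavior Tree task that makes an AI-controlled SCharacter fire a short timed burst from its weapon.
; When the character's BulletCount reaches the reload threshold, it reloads the weapon and resets the count before firing.
; It then starts firing, stops after a brief delay and finishes successfully, or aborts if the pawn is not an SCharacter.
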(event EventReceiveExecuteAI
  (params (OwnerController :type AI%20Controller%20Object%20Reference) (ControlledPawn :type Pawn%20Object%20Reference))
  (bind _asscharacter (Utilities|Casting|CastToSCharacter ControlledPawn)
    (:then
      (if (< (Variables|/Script/HordeGame.SCharacter|GetBulletCount _asscharacter) 100)
        _
        (else
          (Class|SCharacter|ReloadWeapon _asscharacter)
          (Variables|/Script/HordeGame.SCharacter|SetBulletCount _asscharacter 0)))
      (Class|SCharacter|StartFire _asscharacter)
      (Utilities|FlowControl|Delay 0.4)
      (Class|SCharacter|StopFire _asscharacter)
      (AI|BehaviorTree|FinishExecute true))
    (:CastFailed
      (Class|BTTaskBlueprintBase|FinishAbort))))