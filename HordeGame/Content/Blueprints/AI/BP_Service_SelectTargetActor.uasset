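; A behavior tree service that picks an AI pawn's target actor and writes it to a configurable blackboard key.
; Each tick it scans actors known through the pawn's sight perception and skips friendlies and those with no remaining SHealthComponent health.
; The nearest remaining actor becomes the target, and the key is set to none when no candidate qualifies.
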(event EventReceiveTickAI
  (params (OwnerController :type AI%20Controller%20Object%20Reference) (ControlledPawn :type Pawn%20Object%20Reference) (DeltaSeconds :type Float%20%28single-precision%29))
  (Variables|Default|SetBestTargetActor 0)
  (Variables|Default|SetNearestTargetDistance 1e+07)
  (for _array_element (Class|AIPerceptionComponent|GetKnownPerceivedActors (Actor|GetComponentbyClass ControlledPawn "/Script/AIModule.AIPerceptionComponent") "/Script/AIModule.AISense_Sight")
    (if (and (not (Class|SHealthComponent|IsFriendly _array_element ControlledPawn)) (> (Variables|/Script/HordeGame.SHealthComponent|GetCurrentHealth (Actor|GetComponentbyClass _array_element "/Script/HordeGame.SHealthComponent")) 0.0))
      (if (< (Math|Vector|VectorLength (- (Transformation|GetActorLocation ControlledPawn) (Transformation|GetActorLocation _array_element))) (Variables|Default|GetNearestTargetDistance))
        (Variables|Default|SetNearestTargetDistance (Math|Vector|VectorLength (- (Transformation|GetActorLocation ControlledPawn) (Transformation|GetActorLocation _array_element))))
        (Variables|Default|SetBestTargetActor _array_element))))
  (Class|BTFunctionLibrary|SetBlackboardValueasObject (Variables|Default|GetBlackboardKey) (Variables|Default|GetBestTargetActor)))