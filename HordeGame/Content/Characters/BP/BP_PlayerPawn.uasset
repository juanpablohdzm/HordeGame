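; Player pawn Blueprint that sets up the local HUD and the selected hero's appearance when play begins.
; It casts the game instance to HordeGameGameInstance, then adds crosshair and health logo widgets only for a locally controlled pawn.
; For every pawn, a switch on that game instance's character type applies the mesh, materials and animation Blueprint for Belica, Twinblast, Wraith or Mannequin.
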(event EventBeginPlay
  (bind _mesh (Variables|Character|GetMesh))
  (bind _mesh_2 (Variables|Character|GetMesh))
  (bind _mesh_3 (Variables|Character|GetMesh))
  (bind _mesh_4 (Variables|Character|GetMesh))
  (bind _ashorde_game_game_instance (Utilities|Casting|CastToHordeGameGameInstance (Game|GetGameInstance)))
  (Utilities|FlowControl|Sequence
    (:then_0
      ;[1 1 1] Set UI elements
      (if (Pawn|IsLocallyControlled)
        (Utilities|FlowControl|Sequence
          (:then_0
            (bind _returnvalue (UserInterface|CreateWidget "/Game/UI/BP/WBP_CrossHair.WBP_CrossHair_C"))
            (UserInterface|Viewport|AddtoViewport _returnvalue 0))
          (:then_1
            (bind _returnvalue_2 (UserInterface|CreateWidget "/Game/UI/BP/WBP_HealthLogo.WBP_HealthLogo_C"))
            (UserInterface|Viewport|AddtoViewport _returnvalue_2 0)))))
    (:then_1
      (switch Utilities|FlowControl|Switch|SwitchonECharacterType (Class|HordeGameGameInstance|GetCharacterType _ashorde_game_game_instance)
        (:CT_BELICA
          ;[1 1 1] Set character mesh
          (Class|SkinnedMeshComponent|SetSkeletalMesh (Variables|Character|GetMesh) "/Game/Characters/CharacterLtBelica/Meshes/Belica.Belica" true)
          (Rendering|Material|SetMaterial _mesh 0 "/Game/Characters/CharacterLtBelica/Materials/M_Belica_UpperBody.M_Belica_UpperBody")
          (Rendering|Material|SetMaterial _mesh 1 "/Game/Characters/CharacterLtBelica/Materials/M_Belica_LowerBody_Inst.M_Belica_LowerBody_Inst")
          (Components|SkeletalMesh|SetAnimInstanceClass (Variables|Character|GetMesh) "/Game/Characters/CharacterLtBelica/Animations/Belica_AnimBlueprint.Belica_AnimBlueprint_C"))
        (:CT_TWINBLAST
          (Class|SkinnedMeshComponent|SetSkeletalMesh (Variables|Character|GetMesh) "/Game/Characters/CharacterTwinblast/Meshes/TwinBlast.TwinBlast" true)
          (Rendering|Material|SetMaterial _mesh_4 0 "/Game/Characters/CharacterTwinblast/Materials/M_TwinBlast_Head_Shirt.M_TwinBlast_Head_Shirt")
          (Rendering|Material|SetMaterial _mesh_4 1 "/Game/Characters/CharacterTwinblast/Materials/M_TwinBlast_Coat.M_TwinBlast_Coat")
          (Components|SkeletalMesh|SetAnimInstanceClass (Variables|Character|GetMesh) "/Game/Characters/CharacterTwinblast/Animations/Twinblast_AnimBlueprint.Twinblast_AnimBlueprint_C"))
        (:CT_WRAITH
          (Class|SkinnedMeshComponent|SetSkeletalMesh (Variables|Character|GetMesh) "/Game/Characters/CharacterWaith/Meshes/Wraith.Wraith" true)
          (Rendering|Material|SetMaterial _mesh_3 0 "/Game/Characters/CharacterWaith/Materials/M_Wraith_Upperbody.M_Wraith_Upperbody")
          (Rendering|Material|SetMaterial _mesh_3 1 "/Game/Characters/CharacterWaith/Materials/M_Wraith_Lowerbody.M_Wraith_Lowerbody")
          (Components|SkeletalMesh|SetAnimInstanceClass _mesh_3 "/Game/Characters/CharacterWaith/Animations/Wraith_AnimBlueprint.Wraith_AnimBlueprint_C"))
        (:CT_MANNEQUIN
          (Class|SkinnedMeshComponent|SetSkeletalMesh (Variables|Character|GetMesh) "/Game/AnimStarterPack/UE4_Mannequin/Mesh/SK_Mannequin.SK_Mannequin" true)
          (Rendering|Material|SetMaterial _mesh_2 0 "/Game/AnimStarterPack/UE4_Mannequin/Materials/M_UE4Man_Body_Inst.M_UE4Man_Body_Inst")
          (Rendering|Material|SetMaterial _mesh_2 1 "/Game/AnimStarterPack/UE4_Mannequin/Materials/M_UE4Man_ChestLogo_Inst.M_UE4Man_ChestLogo_Inst")
          (Components|SkeletalMesh|SetAnimInstanceClass _mesh_2 "/Game/AnimStarterPack/UE4ASP_HeroTPP_AnimBlueprint.UE4ASP_HeroTPP_AnimBlueprint_C"))))))

(fn ConstructionScript)