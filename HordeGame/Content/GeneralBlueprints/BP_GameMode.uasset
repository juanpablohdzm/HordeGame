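; Game mode Blueprint that spawns AI bots and awards score to killers of non-player pawns.
; SpawnNewBot runs an EQS query for a spawn location, randomly picked from the best 25 percent.
; On query success, a weighted roll favors BP_Character_AI over BP_TrackerBot, and spawning is skipped if collision cannot be resolved.
; An actor-killed binding made at BeginPlay adds points to the killer's SPlayerState.
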(event Custom|SpawnBot
  (params (QueryInstance :type Env%20Query%20Instance%20Blueprint%20Wrapper%20Object%20Reference) (QueryStatus :type EEnvQueryStatus%20Enum :default "Processing"))
  (switch Utilities|FlowControl|Switch|SwitchonEEnvQueryStatus QueryStatus
    (:Success
      (for _array_element (Class|EnvQueryInstanceBlueprintWrapper|GetResultsasLocations QueryInstance)
        (Game|SpawnActorfromClass (select (<= (Math|Random|RandomFloatinRange 0.0 1e+02) 7e+01) "/Game/AI/AI_Character_BP/BP_Character_AI.BP_Character_AI_C" "/Game/AI/TrackerBot/BP_TrackerBot.BP_TrackerBot_C") (Math|Transform|MakeTransform _array_element) "AdjustIfPossibleButDontSpawnIfColliding" 0 0)))))

(event Custom|OnActorKilled_Event
  (params (VictimActor :type Actor%20Object%20Reference) (KillerActor :type Actor%20Object%20Reference) (KillerController :type Controller%20Object%20Reference))
  (bind _aspawn (Utilities|Casting|CastToPawn VictimActor))
  (if (not (Pawn|IsPlayerControlled _aspawn))
    (bind _assplayer_state (Utilities|Casting|CastToSPlayerState (Variables|/Script/Engine.Pawn|GetPlayerState (Pawn|GetControlledPawn KillerController))))
    (Class|SPlayerState|AddScore _assplayer_state 2e+01)))

(event EventBeginPlay
  (EventDispatchers|BindEventtoOnActorKilled (delegate Custom|OnActorKilled_Event)))

(event EventSpawnNewBot
  (bind _returnvalue (AI|EQS|RunEQSQuery "/Game/AI/EQS_FindSpawnLocation.EQS_FindSpawnLocation" self "RandomBest25Pct"))
  (EventDispatchers|AssignOnQueryFinishedEvent _returnvalue (delegate Custom|SpawnBot)))

(fn ConstructionScript)